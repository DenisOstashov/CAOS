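; Door actor that reports player interaction to the quest system, with no opening or movement logic in its graphs.
; On Interact, if flagged as a quest item, it casts the player character to MainCharacterBP and loops through its QuestLog.
; Each incomplete quest receives CallInteracted with the door as the argument.
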(event `/Game/Blueprints/QuestSystem/InteractInterface.Interact`
  (if (`self.IsQuestItem`)
    (bind _asmain_character_bp (cast `/Game/Blueprints/MainCharacter/MainCharacterBP` (`GameplayStatics.GetPlayerCharacter` 0)))
    (for _array_element (`/Game/Blueprints/QuestSystem/QuestLog.Quests` (`/Game/Blueprints/MainCharacter/MainCharacterBP.QuestLog` _asmain_character_bp))
      (if (not (`/Game/Blueprints/QuestSystem/Quests/Quest.IsCompleted` _array_element))
        (`/Game/Blueprints/QuestSystem/Quests/Quest.Interacted` _array_element self)))))

(fn `UserConstructionScript`)