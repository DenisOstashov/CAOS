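; Game instance that holds the player's save data and handles loading, clearing and deleting the save slot.
; On init it loads the MainSaveGame from the configured slot, or creates a fresh save object if none exists.
; LoadLevel opens the level whose name is at the saved CurrentLevel index in the LevelNames array.
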(event `self.ReceiveInit`
  (bind _returnvalue (`GameplayStatics.DoesSaveGameExist` (`self.SaveSlotName`)))
  (if _returnvalue
    (bind _returnvalue_2 (`GameplayStatics.LoadGameFromSlot` (`self.SaveSlotName`)))
    (bind _asmain_save_game (cast `/Game/Blueprints/MainSaveGame` _returnvalue_2))
    (set `self.SaveData` _asmain_save_game)
    (else
      (`self.ClearSaveData`))))

(fn `ClearSaveData`
  (bind _returnvalue (`GameplayStatics.CreateSaveGameObject` "/Game/Blueprints/MainSaveGame.MainSaveGame_C"))
  (set `self.SaveData` _returnvalue))

(fn `DeleteSave`
  (`GameplayStatics.DeleteGameInSlot` (`self.SaveSlotName`)))

(fn `LoadLevel`
  (`GameplayStatics.OpenLevel` (`|GetArrayItem` (`self.LevelNames`) (`/Game/Blueprints/MainSaveGame.CurrentLevel` (`self.SaveData`)))))